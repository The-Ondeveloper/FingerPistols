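; Health component that tracks an owning actor's health and reduces it when that actor takes damage.
; On BeginPlay it binds to the owner's OnTakeAnyDamage, and the damage handler subtracts damage and caps health at the maximum.
; Reaching zero or below only prints a debug "Dead" message, with no death logic here.
; GetHealth exposes the current value to other Blueprints.
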(event `self.ReceiveBeginPlay`
  (add `Actor.OnTakeAnyDamage` (`self.GetOwner`) (`|CreateDelegate` :!event `Update Health`))
  (`KismetSystemLibrary.PrintString` "boom"))

(event `Update Health`
  (params (DamagedActor :type "Actor Object Reference") (Damage :type "Float (single-precision)") (DamageType :type "DamageType Object Reference") (InstigatedBy :type "Controller Object Reference") (DamageCauser :type "Actor Object Reference"))
  (bind _output_get (set `self.CurrentHealth` (- (`self.CurrentHealth`) Damage)))
  (`KismetSystemLibrary.PrintString` (`KismetStringLibrary.Conv_IntToString` _output_get))
  (`|ExecutionSequence`
    (:`then_0`
      (if (> (`self.CurrentHealth`) (`self.MaxHealth`))
        (set `self.CurrentHealth` (`self.MaxHealth`))))
    (:`then_1`
      (if (<= (`self.CurrentHealth`) 0)
        (`KismetSystemLibrary.PrintString` "Dead" true true (struct :`R` 1.0 :`G` 0.018841 :`B` 0.078564 :`A` 1.0))))))

(fn `GetHealth`
  (returns (Health :type Integer))
  (return (`self.CurrentHealth`)))