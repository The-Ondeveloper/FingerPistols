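; BP_ZipPoint is an obstacle actor that flings a character toward itself, acting as a zip point.
; OverlapEvent launches the character at high speed along a look-at direction to the actor, calls InteractionEventMessage on it, then starts a timed cooldown that blocks retriggering.
; A separate ActorBeginOverlap handler applies a negligible launch and prints a debug "Hello", apparently leftover test logic.
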(event `self.ReceiveActorBeginOverlap`
  (params (OtherActor :type "Actor Object Reference"))
  (bind _ascharacter (cast `Character` OtherActor))
  (`Character.LaunchCharacter` _ascharacter (1.0 1.0 1.0) true true)
  (`KismetSystemLibrary.PrintString` "Hello"))

(event `/Game/Projectile/BPI_Interact.OverlapEvent`
  (params (`Other Actor` :type "Actor Object Reference"))
  (if (not (`self.Cooldown`))
    (bind _ascharacter (cast `Character` `Other Actor`))
    (`Character.LaunchCharacter` _ascharacter (* (`KismetMathLibrary.GetForwardVector` (`KismetMathLibrary.FindLookAtRotation` (`self.K2_GetActorLocation` `Other Actor`) (`self.K2_GetActorLocation`))) 10000.0) true true)
    (message `/Game/Obstacles/BPI_Character.Interaction Event` _ascharacter)
    (set `self.Cooldown` true)
    (`KismetSystemLibrary.K2_SetTimerDelegate` (delegate `Reset Cooldown`) (`self.Cooldown Duration`))))

(event `Reset Cooldown`
  (set `self.Cooldown` false))

(fn `UserConstructionScript`)