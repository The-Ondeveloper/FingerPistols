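; Boost pad obstacle that launches any Character overlapping it along the pad component's forward vector, scaled by Power.
; The launch overrides the character's existing velocity on all axes.
; A Cooldown flag blocks further launches after each boost, and a timer set to looping, rather than one-shot, clears it every CooldownDuration.
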(event `self.ReceiveActorBeginOverlap`
  (params (OtherActor :type "Actor Object Reference"))
  (`self.OverlapEvent` OtherActor))

(event `/Game/Projectile/BPI_Interact.OverlapEvent`
  (params (`Other Actor` :type "Actor Object Reference"))
  (if (not (`self.Cooldown`))
    (bind _ascharacter (cast `Character` `Other Actor`))
    (`Character.LaunchCharacter` _ascharacter (* (`KismetMathLibrary.GetForwardVector` (`SceneComponent.K2_GetComponentRotation` (`self.BoostPad`))) (`self.Power`)) true true)
    (set `self.Cooldown` true)
    (`KismetSystemLibrary.K2_SetTimerDelegate` (delegate `Reset Cooldown`) (`self.Cooldown Duration`) true)))

(event `Reset Cooldown`
  (set `self.Cooldown` false))

(fn `UserConstructionScript`)