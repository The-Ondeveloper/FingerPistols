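; BP_TransformSwitch is an obstacle switch that moves a referenced actor between its starting transform and a target transform when something overlaps it.
; The construction script captures the actor's transform as the start and adds two arrow components to preview the start and target transforms.
; A Timeline drives the transform lerp, either playing once when HappensOnce is set or alternating forward and reverse on successive overlaps.
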(event `self.ReceiveBeginPlay`)

(event `self.ReceiveActorBeginOverlap`
  (params (OtherActor :type "Actor Object Reference"))
  (if (`self.Happens Once`)
    (`/Engine/EditorBlueprintResources/StandardMacros.DoOnce` false
      (:`Completed`
        (bind (_direction _progression) (`Timeline|Timeline` :!label _label)
          (:`Update`
            (`self.K2_SetActorTransform` (`self.ActorToAffect`) (`KismetMathLibrary.TLerp` (`self.StartTransform`) (`self.TransformChange`) _progression) false false)))))
    (else
      (`/Engine/EditorBlueprintResources/StandardMacros.FlipFlop`
        (:`A`
          (goto _label))
        (:`B`
          (goto _label :!via `Reverse`))))))

(fn `UserConstructionScript`
  (bind _actortoaffect (`self.ActorToAffect`)
    (:`then`
      (`parent.UserConstructionScript`)
      (bind _output_get (set `self.StartTransform` (`self.GetTransform` _actortoaffect)))
      (bind _returnvalue (`AddComponent|NODE_AddArrowComponent-1`))
      (`SceneComponent.K2_SetWorldTransform` _returnvalue _output_get false false)
      (bind _returnvalue_2 (`AddComponent|NODE_AddArrowComponent-0`))
      (`SceneComponent.K2_SetWorldTransform` _returnvalue_2 (`self.TransformChange`) false false))
    (:`else`)))