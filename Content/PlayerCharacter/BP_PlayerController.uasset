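; Player controller that sets up the player's input and score tracking and exposes ability permission flags.
; On BeginPlay, if the Enhanced Input subsystem is valid, it adds the player controls mapping context, fires OnBindingsChanged and spawns a ScoreManager owned by the player character.
; Simple getters return the CanBoost, CanJump and CanShoot flags, which this graph never changes.
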(event `self.ReceiveBeginPlay`
  (bind _returnvalue (subsystem `EnhancedInputLocalPlayerSubsystem`))
  (`/Engine/EditorBlueprintResources/StandardMacros.IsValid` _returnvalue
    (:`Is Valid`
      (`EnhancedInputSubsystemInterface.AddMappingContext` _returnvalue "/Game/PlayerCharacter/Input/MC_PlayerControls.MC_PlayerControls" 0 (struct))
      (`self.OnBindingsChanged`)
      (`|SpawnActorFromClass` "/Game/PlayerCharacter/Components/ScoreManager.ScoreManager_C" (`self.Spawn Transform`) "Undefined" "MultiplyWithRoot" (`GameplayStatics.GetPlayerCharacter` 0) null))))

(fn `Get Can Boost`
  (returns (`Return Value` :type Boolean))
  (return (`self.CanBoost`)))

(fn `Get Can Jump`
  (returns (`Return Value` :type Boolean))
  (return (`self.CanJump`)))

(fn `Get Can Shoot`
  (returns (`Return Value` :type Boolean))
  (return (`self.CanShoot`)))

(fn `UserConstructionScript`)