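; Tutorial game mode that starts the player with boosting, jumping and shooting disabled.
; On BeginPlay it runs the parent logic, then waits one tick before switching off the three abilities through the pistols player controller.
; ResetLevel only calls the parent implementation, so it does not reapply the restrictions itself, and nothing here re-enables them.
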(event `Disable Controls`
  (bind _bp_player_controller (`/Game/CommonFunctionLibrary.GetPistolsPlayerController`))
  (`KismetSystemLibrary.DelayUntilNextTick`)
  (`/Game/PlayerCharacter/BP_PlayerController.Set Can Boost` _bp_player_controller false)
  (`/Game/PlayerCharacter/BP_PlayerController.Set Can Jump` _bp_player_controller false)
  (`/Game/PlayerCharacter/BP_PlayerController.Set Can Shoot` _bp_player_controller false))

(event `self.ReceiveBeginPlay`
  (`parent.ReceiveBeginPlay`)
  (`self.Disable Controls`))

(event `self.Reset Level`
  (`parent.Reset Level`))

(fn `UserConstructionScript`
  (`parent.UserConstructionScript`))